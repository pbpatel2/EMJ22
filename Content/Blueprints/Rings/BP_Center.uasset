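; Center piece of the rings setup that acts as the win trigger once its win condition is enabled.
; EnableWinCondition arms it, after which a BP_ThirdPersonCharacter entering the capsule is sent into ragdoll.
; The same overlap plays a timeline from the start, lerping the static mesh's relative location from its BeginPlay position to LocationTarget as an ascend motion.
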(event `self.ReceiveBeginPlay`
  (bind _returnvalue_location (`KismetMathLibrary.BreakTransform` (`SceneComponent.GetRelativeTransform` (`self.StaticMesh`))))
  (set `self.LocationStart` _returnvalue_location))

(event `self.Capsule.OnComponentBeginOverlap`
  (params (OverlappedComponent :type "PrimitiveComponent Object Reference") (OtherActor :type "Actor Object Reference") (OtherComp :type "PrimitiveComponent Object Reference") (OtherBodyIndex :type Integer) (bFromSweep :type Boolean) (SweepResult :type "HitResult Structure (by ref)"))
  (if (`self.WinConditionActive`)
    (bind _asbp_third_person_character (cast `/Game/ThirdPerson/Blueprints/BP_ThirdPersonCharacter` OtherActor))
    (`/Game/ThirdPerson/Blueprints/BP_ThirdPersonCharacter.Event Ragdoll` _asbp_third_person_character)
    (bind (_direction _alpha) (`Timeline|Ascend Timeline` :!via `PlayFromStart`)
      (:`Update`
        (`SceneComponent.K2_SetRelativeTransform` (`self.StaticMesh`) (`KismetMathLibrary.Conv_VectorToTransform` (`KismetMathLibrary.VLerp` (`self.LocationStart`) (`self.LocationTarget`) _alpha)) false false)))))

(event `Event Enable Win Condition`
  (set `self.WinConditionActive` true))

(fn `UserConstructionScript`)