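; BP_Ring7 is a child ring Blueprint that ties the start of its rotation to the sword spawn volumes in the level.
; It overrides StartRotation to run the parent logic, then finds every BP_SpawnVolumeSwords actor and calls EventRing7Swords on each.
; The event graph holds only disabled default events, and the construction script just calls the parent.
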(fn `StartRotation`
  (`parent.StartRotation`)
  (bind _outactors (`GameplayStatics.GetAllActorsOfClass` "/Game/VFX/BP_SpawnVolumeSwords.BP_SpawnVolumeSwords_C"))
  (for _array_element _outactors
    (`/Game/VFX/BP_SpawnVolumeSwords.Event Ring7 Swords` _array_element)))

(fn `UserConstructionScript`
  (`parent.UserConstructionScript`))