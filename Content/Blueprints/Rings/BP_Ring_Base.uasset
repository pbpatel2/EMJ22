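; Base ring actor that starts spinning once all of its pickup sockets have been filled.
; BeginPlay counts the children of Sockets and copies the ring's static mesh onto a collision mesh component.
; Each OnPickupInsert raises the completed count, calling StartRotation when it matches the socket total.
; EventRotate then re-arms itself on a short timer, applying swept yaw steps; EndRotation is an empty stub.
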(event `/Game/Blueprints/Interfaces/BPI_Socket.OnPickupInsert`
  (`/Engine/EditorBlueprintResources/StandardMacros.IncrementInt` (`self.SocketCompleteCount`)
    (:`  `
      (if (== (`self.SocketCount`) (`self.SocketCompleteCount`))
        (`self.StartRotation`)))))

(event `self.ReceiveBeginPlay`
  (set `self.SocketCount` (`SceneComponent.GetNumChildrenComponents` (`self.Sockets`)))
  (`StaticMeshComponent.SetStaticMesh` (`self.SM_Ring_Collide`) (`StaticMeshComponent.StaticMesh` (`self.SM_Ring`))))

(event `EventRotate`
  (`KismetSystemLibrary.K2_SetTimerDelegate` (delegate `EventRotate`) 0.01 (`self.RotationEnabled`))
  (`self.K2_AddActorWorldRotation` self (`KismetMathLibrary.MakeRotator` 0.0 0.0 (`self.RotationSpeed`)) true false))

(fn `EndRotation`)

(fn `StartRotation`
  (set `self.RotationEnabled` true)
  (`self.EventRotate`))

(fn `UserConstructionScript`)