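; BP_Ring6 is a ring Blueprint that adds a fire event to the rotation inherited from its parent class.
; Its StartRotation override runs the parent logic, plays the fire cue as 2D sound, then calls EventRing6Fire on every BP_SpawnVolumeFire in the level.
; BeginPlay and construction only forward to the parent, and the overlap and Tick events are disabled.
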(event `self.ReceiveBeginPlay`
  (`parent.ReceiveBeginPlay`))

(fn `StartRotation`
  (`parent.StartRotation`)
  (`GameplayStatics.PlaySound2D` "/Game/Audio/Cue_Fire.Cue_Fire" 1.0 1.0 0.0 null null)
  (bind _outactors (`GameplayStatics.GetAllActorsOfClass` "/Game/VFX/BP_SpawnVolumeFire.BP_SpawnVolumeFire_C"))
  (for _array_element _outactors
    (`/Game/VFX/BP_SpawnVolumeFire.Event Ring6 Fire` _array_element)))

(fn `UserConstructionScript`
  (`parent.UserConstructionScript`))