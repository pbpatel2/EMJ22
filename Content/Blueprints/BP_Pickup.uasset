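; BP_Pickup is a pickup actor made of a configurable static mesh and a sphere trigger.
; The construction script applies the mesh and material when the mesh is valid, then sets the sphere radius from TriggerRadius.
; Sphere overlaps send enter and exit messages to the other actor, passing the pickup itself on enter, and contain no collection logic of their own.
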(event `self.Sphere.OnComponentBeginOverlap`
  (params (OverlappedComponent :type "PrimitiveComponent Object Reference") (OtherActor :type "Actor Object Reference") (OtherComp :type "PrimitiveComponent Object Reference") (OtherBodyIndex :type Integer) (bFromSweep :type Boolean) (SweepResult :type "HitResult Structure (by ref)"))
  (message `/Game/Blueprints/Interfaces/BPI_Pickup.OnPickupTriggerEnter` OtherActor self))

(event `self.Sphere.OnComponentEndOverlap`
  (params (OverlappedComponent :type "PrimitiveComponent Object Reference") (OtherActor :type "Actor Object Reference") (OtherComp :type "PrimitiveComponent Object Reference") (OtherBodyIndex :type Integer))
  (message `/Game/Blueprints/Interfaces/BPI_Pickup.OnPickupTriggerExit` OtherActor))

(fn `UserConstructionScript`
  (bind _staticmesh (`self.StaticMesh`))
  (`|ExecutionSequence`
    (:`then_0`
      (`/Engine/EditorBlueprintResources/StandardMacros.IsValid` (`self.Mesh`)
        (:`Is Valid`
          (`StaticMeshComponent.SetStaticMesh` _staticmesh (`self.Mesh`))
          (`PrimitiveComponent.SetMaterial` _staticmesh 0 (`self.Material`)))))
    (:`then_1`
      (`SphereComponent.SetSphereRadius` (`self.Sphere`) (`self.TriggerRadius`) true))))