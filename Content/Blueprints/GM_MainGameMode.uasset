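; Main game mode that tracks player HP and socket completion, shows the HUD, and plays background music.
; On BeginPlay it counts BP_Socket actors; once completed sockets reach that total, it enables the win condition on BP_Center.
; At zero HP, the player ragdolls and drops any pickup, then after a delay respawns at PlayerStart with HP reset.
; An IsDying flag blocks repeated death triggers during the sequence.
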(event `self.ReceiveBeginPlay`
  (`|ExecutionSequence`
    (:`then_0`
      (bind _outactors (`GameplayStatics.GetAllActorsOfClass` "/Game/Blueprints/BP_Socket.BP_Socket_C"))
      (set `self.SocketMax` (`KismetArrayLibrary.Array_Length` _outactors)))
    (:`then_1`
      (`self.Add_Widget`))
    (:`then_2`
      (bind _returnvalue (`GameplayStatics.GetActorOfClass` "/Game/ThirdPerson/Blueprints/BP_ThirdPersonCharacter.BP_ThirdPersonCharacter_C"))
      (set `self.Player` _returnvalue))
    (:`then_3`
      (`GameplayStatics.PrimeSound` "/Game/Audio/Cue_Enchanted_Forest.Cue_Enchanted_Forest")
      (`GameplayStatics.PlaySound2D` "/Game/Audio/Cue_Enchanted_Forest.Cue_Enchanted_Forest" 0.3 1.0 0.0 null null))))

(event `EventPlayerDeath`
  (set `self.IsDying` true)
  (`self.PlayerDeath`)
  (`KismetSystemLibrary.Delay` 2.0)
  (`self.K2_DestroyActor` (`GameplayStatics.GetPlayerCharacter` 0))
  (`self.PlayerRespawn`)
  (set `self.IsDying` false))

(fn `Add_Widget`
  (bind _returnvalue (`|CreateWidget` "/Game/UI/W_HUD.W_HUD_C"))
  (bind _output_get (set `self.HUD` _returnvalue))
  (`UserWidget.AddToViewport` _output_get 0))

(fn `OnSocketComplete`
  (bind _result (`/Engine/EditorBlueprintResources/StandardMacros.IncrementInt` (`self.SocketComplete`))
    (:`  `
      (`/Game/UI/W_HUD.UpdateSocketText` (`self.HUD`))
      (if (>= _result (`self.SocketMax`))
        (bind _returnvalue (`GameplayStatics.GetActorOfClass` "/Game/Blueprints/Rings/BP_Center.BP_Center_C"))
        (`/Game/Blueprints/Rings/BP_Center.Event Enable Win Condition` _returnvalue)))))

(fn `PlayerDeath`
  (`GameplayStatics.PlaySound2D` "/Game/Audio/Cue_Death.Cue_Death" 1.0 1.0 0.0 null null)
  (bind _asbp_third_person_character (cast `/Game/ThirdPerson/Blueprints/BP_ThirdPersonCharacter` (`GameplayStatics.GetPlayerCharacter` 0)))
  (`/Game/ThirdPerson/Blueprints/BP_ThirdPersonCharacter.Event Ragdoll` _asbp_third_person_character)
  (if (`/Game/ThirdPerson/Blueprints/BP_ThirdPersonCharacter.PickupHeld` _asbp_third_person_character)
    (`/Game/ThirdPerson/Blueprints/BP_ThirdPersonCharacter.Drop_Pickup` _asbp_third_person_character)))

(fn `PlayerRespawn`
  (bind _returnvalue (`GameplayStatics.GetActorOfClass` "/Script/Engine.PlayerStart"))
  (bind _returnvalue_2 (`|SpawnActorFromClass` "/Game/ThirdPerson/Blueprints/BP_ThirdPersonCharacter.BP_ThirdPersonCharacter_C" (`KismetMathLibrary.Conv_VectorToTransform` (`SceneComponent.K2_GetComponentLocation` (`Actor.RootComponent` _returnvalue))) "Undefined" "OverrideRootScale" null null))
  (`Controller.Possess` (`GameplayStatics.GetPlayerController` 0) _returnvalue_2)
  (bind _output_get (set `self.Player` _returnvalue_2))
  (`/Game/ThirdPerson/Blueprints/BP_ThirdPersonCharacter.Event Disable Ragdoll` _output_get)
  (`self.UpdatePlayerHP` (- 5 (`self.PlayerHP`))))

(fn `UpdatePlayerHP`
  (params (HPDelta :type Integer))
  (bind _output_get (set `self.PlayerHP` (+ (`self.PlayerHP`) HPDelta)))
  (`/Game/UI/W_HUD.UpdateHPText` (`self.HUD`))
  (if (and (<= _output_get 0) (not (`self.IsDying`)))
    (`self.EventPlayerDeath`)))

(fn `UserConstructionScript`
  (set `self.DefaultPawnClass` "/Game/ThirdPerson/Blueprints/BP_ThirdPersonCharacter.BP_ThirdPersonCharacter_C"))