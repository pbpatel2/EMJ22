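; BP_Socket is a receptacle that accepts pickups and reports its completion to the main game mode.
; Its trigger sphere, sized from TriggerRadius at construction, messages overlapping actors on enter and exit, passing itself on enter.
; InsertPickup disables the pickup's collision, snaps and attaches it to PickupTarget, then notifies the first RingClass actor and GM_MainGameMode.
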(event `self.ReceiveBeginPlay`)

(event `self.Sphere.OnComponentBeginOverlap`
  (params (OverlappedComponent :type "PrimitiveComponent Object Reference") (OtherActor :type "Actor Object Reference") (OtherComp :type "PrimitiveComponent Object Reference") (OtherBodyIndex :type Integer) (bFromSweep :type Boolean) (SweepResult :type "HitResult Structure (by ref)"))
  (message `/Game/Blueprints/Interfaces/BPI_Socket.OnSocketTriggerEnter` OtherActor self))

(event `self.Sphere.OnComponentEndOverlap`
  (params (OverlappedComponent :type "PrimitiveComponent Object Reference") (OtherActor :type "Actor Object Reference") (OtherComp :type "PrimitiveComponent Object Reference") (OtherBodyIndex :type Integer))
  (message `/Game/Blueprints/Interfaces/BPI_Socket.OnSocketTriggerExit` OtherActor))

(fn `InsertPickup`
  (params (Pickup :type "/Game/Blueprints/BP_Pickup Object Reference"))
  (bind _pickuptarget (`self.PickupTarget`))
  (`PrimitiveComponent.SetCollisionProfileName` (`/Game/Blueprints/BP_Pickup.Sphere` Pickup) "NoCollision" true)
  (`self.K2_SetActorTransform` Pickup (`SceneComponent.K2_GetComponentToWorld` _pickuptarget) true false)
  (`self.K2_AttachToComponent` Pickup _pickuptarget "None" "SnapToTarget" "SnapToTarget" "SnapToTarget" false)
  (bind _outactors (`GameplayStatics.GetAllActorsOfClass` (`self.RingClass`)))
  (message `/Game/Blueprints/Interfaces/BPI_Socket.OnPickupInsert` (`|GetArrayItem` _outactors))
  (bind _asgm_main_game_mode (cast `/Game/Blueprints/GM_MainGameMode` (`GameplayStatics.GetGameMode`)))
  (`/Game/Blueprints/GM_MainGameMode.OnSocketComplete` _asgm_main_game_mode))

(fn `UserConstructionScript`
  (`SphereComponent.SetSphereRadius` (`self.Sphere`) (`self.TriggerRadius`) true))