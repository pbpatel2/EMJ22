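; BP_Sword is a falling sword hazard that damages the player on contact.
; On spawn it drives its Cone through ProjectileMovement, waits briefly, launches straight down, then destroys itself after a further delay.
; When the Cone overlaps BP_ThirdPersonCharacter, it subtracts one HP through GM_MainGameMode and destroys itself.
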(event `self.ReceiveBeginPlay`
  (bind _projectilemovement (`self.ProjectileMovement`))
  (`MovementComponent.SetUpdatedComponent` _projectilemovement (`self.Cone`))
  (`KismetSystemLibrary.Delay` 2.0)
  (set `MovementComponent.Velocity` (0.0 0.0 -1000.0) _projectilemovement)
  (`KismetSystemLibrary.Delay` 3.0)
  (`self.K2_DestroyActor`))

(event `self.Cone.OnComponentBeginOverlap`
  (params (OverlappedComponent :type "PrimitiveComponent Object Reference") (OtherActor :type "Actor Object Reference") (OtherComp :type "PrimitiveComponent Object Reference") (OtherBodyIndex :type Integer) (bFromSweep :type Boolean) (SweepResult :type "HitResult Structure (by ref)"))
  (cast `/Game/ThirdPerson/Blueprints/BP_ThirdPersonCharacter` OtherActor)
  (bind _asgm_main_game_mode (cast `/Game/Blueprints/GM_MainGameMode` (`GameplayStatics.GetGameMode`)))
  (`/Game/Blueprints/GM_MainGameMode.UpdatePlayerHP` _asgm_main_game_mode -1)
  (`self.K2_DestroyActor`))

(fn `UserConstructionScript`)